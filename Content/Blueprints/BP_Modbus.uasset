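; BP_Modbus is a test Blueprint that polls a device over Modbus RTU on a serial port and prints the returned values.
; BeginPlay opens the connection and binds the read-complete event, while Tick requests a block of holding registers every frame.
; EndPlay calls the TCP close function on the RTU connection.
; Unwired nodes show alternative TCP connections and a single-register write.
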(event Custom|Event
  (params (Success :type Boolean) (Result :type Array%20of%20Integers))
  (if Success
    (for _array_element Result
      (Development|PrintString (Utilities|String|ToString(Integer) _array_element)))))

(event EventBeginPlay
  ;[1 1 1] serial port
  (bind _returnvalue (Class|UnrealModbusLibrary|CreateModbusRTUConnection "COM1" 9600 "None" 8 1 1))
  (bind _output_get (Variables|Default|SetModbusConnection _returnvalue))
  (Utilities|IsValid _output_get
    (:Is%20Valid
      (Development|PrintString "ModbusConnection success")
      (Utilities|FlowControl|Delay 0.2)
      (EventDispatchers|BindEventtoOnReadHoldingRegistersComplete _output_get (delegate Custom|Event)))
    (:Is%20Not%20Valid
      (Development|PrintString "ModbusConnection fail"))))

(event EventEndPlay
  (params (EndPlayReason :type EEndPlayReason%20Enum :default "Destroyed"))
  (Class|UnrealModbusLibrary|CloseModbusTCPConnection (Variables|Default|GetModbusConnection)))

(event EventTick
  (params (DeltaSeconds :type Float%20%28single-precision%29))
  (bind _modbusconnection (Variables|Default|GetModbusConnection))
  (Utilities|IsValid _modbusconnection
    (:Is%20Valid
      ;[1 1 1] read operation
      (Class|UnrealModbusLibrary|ReadHoldingRegisters _modbusconnection 0 10))))

(fn ConstructionScript)